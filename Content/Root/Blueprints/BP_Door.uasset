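; BP_Door is a two-panel door that opens automatically when the player character approaches and closes when they leave.
; A Trigger component's begin and end overlaps, filtered by a cast to CorePlayerCharacter, play and reverse a timeline.
; The timeline's DoorOpen track lerps the relative locations of the Left and Right components, each between its own begin and end vectors.
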(event OnComponentEndOverlap(Trigger)
  (params (OverlappedComponent :type Primitive%20Component%20Object%20Reference) (OtherActor :type Actor%20Object%20Reference) (OtherComp :type Primitive%20Component%20Object%20Reference) (OtherBodyIndex :type Integer))
  (Utilities|Casting|CastToCorePlayerCharacter OtherActor)
  (bind _door_open (Timeline|Timeline_0 Reverse)
    (:Update
      (Transformation|SetRelativeLocation (Variables|Default|GetRight) (Math|Vector|Lerp(Vector) (Variables|Default|GetBegin) (Variables|Default|GetEnd) _door_open) false false)
      (Transformation|SetRelativeLocation (Variables|Default|GetLeft) (Math|Vector|Lerp(Vector) (Variables|Default|GetBegin2) (Variables|Default|GetEnd2) _door_open) false false))))

(event OnComponentBeginOverlap(Trigger)
  (params (OverlappedComponent :type Primitive%20Component%20Object%20Reference) (OtherActor :type Actor%20Object%20Reference) (OtherComp :type Primitive%20Component%20Object%20Reference) (OtherBodyIndex :type Integer) (bFromSweep :type Boolean) (SweepResult :type Hit%20Result%20Structure%20%28by%20ref%29))
  (Utilities|Casting|CastToCorePlayerCharacter OtherActor)
  (bind _door_open (Timeline|Timeline_0 Play)
    (:Update
      (Transformation|SetRelativeLocation (Variables|Default|GetRight) (Math|Vector|Lerp(Vector) (Variables|Default|GetBegin) (Variables|Default|GetEnd) _door_open) false false)
      (Transformation|SetRelativeLocation (Variables|Default|GetLeft) (Math|Vector|Lerp(Vector) (Variables|Default|GetBegin2) (Variables|Default|GetEnd2) _door_open) false false))))

(fn ConstructionScript)