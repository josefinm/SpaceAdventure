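; BP_DoorKeycard is a sliding double door that opens only when the player holds a keycard.
; When the FirstPersonCharacter enters the trigger, it checks HasKeycard on BP_GameInstance and plays two timelines that lerp the Right and Left panels between begin and end positions.
; Leaving the trigger reverses both timelines to close the door, without rechecking the keycard.
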(event OnComponentEndOverlap(Trigger)
  (params (OverlappedComponent :type Primitive%20Component%20Object%20Reference) (OtherActor :type Actor%20Object%20Reference) (OtherComp :type Primitive%20Component%20Object%20Reference) (OtherBodyIndex :type Integer))
  (Utilities|Casting|CastToFirstPersonCharacter OtherActor)
  (Utilities|FlowControl|Sequence
    (:then_0
      (bind _door_open (Timeline|Timeline_0 Reverse)
        (:Update
          (Transformation|SetRelativeLocation (Variables|Default|GetRight) (Math|Vector|Lerp(Vector) (Variables|Default|GetBegin) (Variables|Default|GetEnd) _door_open) false false))))
    (:then_1
      (bind _door_open_2 (Timeline|Timeline_1 Reverse)
        (:Update
          (Transformation|SetRelativeLocation (Variables|Default|GetLeft) (Math|Vector|Lerp(Vector) (Variables|Default|GetBegin2) (Variables|Default|GetEnd2) _door_open_2) false false))))))

(event OnComponentBeginOverlap(Trigger)
  (params (OverlappedComponent :type Primitive%20Component%20Object%20Reference) (OtherActor :type Actor%20Object%20Reference) (OtherComp :type Primitive%20Component%20Object%20Reference) (OtherBodyIndex :type Integer) (bFromSweep :type Boolean) (SweepResult :type Hit%20Result%20Structure%20%28by%20ref%29))
  (Utilities|Casting|CastToFirstPersonCharacter OtherActor)
  (bind _asbp_game_instance (Utilities|Casting|CastToBP_GameInstance (Game|GetGameInstance)))
  (if (Variables|/Game/BP_GameInstance.BP_GameInstance_C|GetbHasKeycard _asbp_game_instance)
    (Utilities|FlowControl|Sequence
      (:then_0
        (bind _door_open (Timeline|Timeline_0 Play)
          (:Update
            (Transformation|SetRelativeLocation (Variables|Default|GetRight) (Math|Vector|Lerp(Vector) (Variables|Default|GetBegin) (Variables|Default|GetEnd) _door_open) false false))))
      (:then_1
        (bind _door_open_2 (Timeline|Timeline_1 Play)
          (:Update
            (Transformation|SetRelativeLocation (Variables|Default|GetLeft) (Math|Vector|Lerp(Vector) (Variables|Default|GetBegin2) (Variables|Default|GetEnd2) _door_open_2) false false)))))))

(fn ConstructionScript)